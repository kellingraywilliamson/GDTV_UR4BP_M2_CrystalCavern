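; BP_PlayerPawn is a player pawn that moves by rolling a physics-driven sphere.
; Forward/backward and right/left input axes apply torque to the Sphere on Y and X respectively, scaled by TorqueMultiplier.
; The torque is applied as an acceleration change, so it ignores the sphere's mass.
; On BeginPlay, the player camera fades in from full opacity.
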(event `self.ReceiveBeginPlay`
  ;[0.3852 0.2817 1] Fade in on start
  (`PlayerCameraManager.StartCameraFade` :`self` (`GameplayStatics.GetPlayerCameraManager` 0) :`FromAlpha` 1.0 :`ToAlpha` 0.0 :`Duration` 1.0))

(event `InputAxis|Move Forward/Backwards`
  (params (AxisValue :type "Float (single-precision)"))
  ;[1 1 1] Forward/Backward Movement
  (`PrimitiveComponent.AddTorqueInRadians` (`self.Sphere`) (`KismetMathLibrary.MakeVector` 0.0 (* AxisValue (`self.TorqueMultiplier`))) "None" true))

(event `InputAxis|Move Right/Left`
  (params (AxisValue :type "Float (single-precision)"))
  ;[1 1 1] Right/Left Movement
  (`PrimitiveComponent.AddTorqueInRadians` (`self.Sphere`) (`KismetMathLibrary.MakeVector` (* AxisValue (`self.TorqueMultiplier`))) "None" true))

(fn `UserConstructionScript`)